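; Rifle projectile for a SuperHot-style game that spins in flight and shatters on impact.
; On spawn it briefly sets global time dilation to half speed, then applies the TimeDilationControl value from the game instance.
; On hit it spawns and triggers an FS_MasterField field system at the impact point, enables physics on the GCRifle component, and destroys itself after a short delay.
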(event `self.ReceiveBeginPlay`
  (bind _asbp_time_dilation_variable (cast `/Game/aSuperHot/Blueprints/BP_TimeDilationVariable` (`GameplayStatics.GetGameInstance`)))
  (`GameplayStatics.SetGlobalTimeDilation` 0.5)
  (`KismetSystemLibrary.Delay` 0.1)
  (`GameplayStatics.SetGlobalTimeDilation` (`/Game/aSuperHot/Blueprints/BP_TimeDilationVariable.TimeDilationControl` _asbp_time_dilation_variable)))

(event `self.ReceiveTick`
  (params (DeltaSeconds :type "Float (single-precision)"))
  (`self.K2_AddActorLocalRotation` (struct :`Pitch` -0.5 :`Roll` -0.5)))

(event `self.ReceiveHit`
  (params (MyComp :type "PrimitiveComponent Object Reference") (Other :type "Actor Object Reference") (OtherComp :type "PrimitiveComponent Object Reference") (bSelfMoved :type Boolean) (HitLocation :type "Vector Structure") (HitNormal :type "Vector Structure") (NormalImpulse :type "Vector Structure") (Hit :type "HitResult Structure (by ref)"))
  (bind _returnvalue (`|SpawnActorFromClass` "/Engine/EditorResources/FieldNodes/FS_MasterField.FS_MasterField_C" (`KismetMathLibrary.MakeTransform` HitLocation) "Undefined" "MultiplyWithRoot" null null))
  (set `/Engine/EditorResources/FieldNodes/FS_MasterField.ActivationType` "NewEnumerator4" _returnvalue)
  (`/Engine/EditorResources/FieldNodes/FS_MasterField.CE_Trigger` _returnvalue)
  (`PrimitiveComponent.SetSimulatePhysics` (`self.GC_Rifle`) true)
  (`KismetSystemLibrary.Delay` 2.0)
  (`self.K2_DestroyActor`))

(fn `UserConstructionScript`)