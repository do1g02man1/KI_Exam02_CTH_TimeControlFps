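; Behavior tree service that keeps an AI pawn's distance to the player up to date on the blackboard.
; On each tick it prints the stored distance, then, if the target actor key holds a valid object, writes a freshly computed value to the distance key.
; The target actor only gates the update, as the distance is always measured to player pawn 0.
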(event `self.ReceiveTickAI`
  (params (OwnerController :type "AIController Object Reference") (ControlledPawn :type "Pawn Object Reference") (DeltaSeconds :type "Float (single-precision)"))
  (`KismetSystemLibrary.PrintString` (`KismetStringLibrary.Conv_DoubleToString` (`BTFunctionLibrary.GetBlackboardValueAsFloat` (`self.TargetDistanceKey`))))
  (`/Engine/EditorBlueprintResources/StandardMacros.IsValid` (`BTFunctionLibrary.GetBlackboardValueAsObject` (`self.TargetActorKey`))
    (:`Is Valid`
      (`BTFunctionLibrary.SetBlackboardValueAsFloat` (`self.TargetDistanceKey`) (`KismetMathLibrary.VSize` (- (`Actor.K2_GetActorLocation` ControlledPawn) (`Actor.K2_GetActorLocation` (`GameplayStatics.GetPlayerPawn` 0))))))))